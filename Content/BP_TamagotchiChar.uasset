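; Tamagotchi-style pet character whose hunger and fun stats drain over time, destroying it when either runs out.
; BeginPlay shows the cursor, creates the UMG_PlayerInteract widget with a self reference, and starts two looping Delay timers that check Death before each decrement.
; IncreseHunger and IncreaseFun top up the stats with clamping, while CheckMood turns them into status text; none are called within this Blueprint.
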(event `self.ReceiveBeginPlay`
  (set `PlayerController.bShowMouseCursor` true (`GameplayStatics.GetPlayerController` 0))
  (bind _returnvalue (`|CreateWidget` "/Game/UMG_PlayerInteract.UMG_PlayerInteract_C" null self))
  (`UserWidget.AddToViewport` _returnvalue 0)
  (`self.Hunger`)
  (`self.Fun`))

(event `Hunger`
  (bind _returnvalue (- (`self.CurrentHunger`) 1))
  (`KismetSystemLibrary.Delay` 0.2 :!label _label)
  (`self.Death` _returnvalue (- (`self.CurrentFun`) 1))
  (set `self.CurrentHunger` _returnvalue)
  (goto _label))

(event `Fun`
  (bind _returnvalue (- (`self.CurrentFun`) 1))
  (`KismetSystemLibrary.Delay` 0.2 :!label _label_2)
  (`self.Death` (- (`self.CurrentHunger`) 1) _returnvalue)
  (set `self.CurrentFun` _returnvalue)
  (goto _label_2))

(fn `CheckMood`
  (bind _currenthunger (`self.CurrentHunger`))
  (bind _currentfun (`self.CurrentFun`))
  (if (or (<= _currenthunger 0) (<= _currentfun 0))
    (set `self.CurrentMood` "GAME OVER")
    (elif (or (<= _currenthunger 50) (<= _currentfun 50))
      (set `self.CurrentMood` "Looks like you're going to loose")
      (elif (or (> _currenthunger 50) (> _currentfun 50))
        (set `self.CurrentMood` "Looks like you're doing well.")
        (else
          (set `self.CurrentMood` "Somethings not right"))))))

(fn `Death`
  (params (HungerIndex :type Integer) (FunIndex :type Integer))
  (if (or (<= HungerIndex 0) (<= FunIndex 0))
    (set `self.CurrentMood` "DEAD")
    (`self.K2_DestroyActor`)))

(fn `IncreaseFun`
  (set `self.CurrentFun` (`KismetMathLibrary.Clamp` (+ (`self.CurrentFun`) 20) 0 100)))

(fn `IncreseHunger`
  (set `self.CurrentHunger` (`KismetMathLibrary.Clamp` (+ (`self.CurrentHunger`) 20) 0 100)))

(fn `UserConstructionScript`)